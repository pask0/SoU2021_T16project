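; Pillar destruction Blueprint that repeatedly places a random explosion on its static meshes, apparently to drive vertex-animated destruction in their materials.
; After BeginPlay, a timed loop picks a point within mesh bounds and a random radius, then moves and resizes a sphere to match.
; Each mesh receives the local-space position, with Z clamped, and radius through Custom Primitive Data.
; The construction script writes the same data with a fixed radius.
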(event `self.ReceiveBeginPlay`
  (bind _sphere (`self.Sphere`))
  (bind _staticmesharray (`self.StaticMeshArray`))
  (bind (_origin _boxextent) (`KismetSystemLibrary.GetComponentBounds` (`|GetArrayItem` _staticmesharray (`KismetMathLibrary.RandomIntegerInRange` 0 (`KismetArrayLibrary.Array_LastIndex` _staticmesharray)))))
  (`KismetSystemLibrary.Delay` 0.1)
  (set `self.ExplosionPos` (`KismetMathLibrary.RandomPointInBoundingBox` _origin _boxextent) :!label _label)
  (set `self.ExplosionRadius` (`KismetMathLibrary.RandomFloatInRange` 25.0 100.0))
  (`SphereComponent.SetSphereRadius` _sphere (`self.ExplosionRadius`) true)
  (`SceneComponent.K2_SetWorldLocation` _sphere (`self.ExplosionPos`) false false)
  (for _array_element (`self.StaticMeshArray`)
    (`PrimitiveComponent.SetCustomPrimitiveDataVector4` _array_element 0 (`KismetMathLibrary.MakeVector4` (.x (`KismetMathLibrary.InverseTransformLocation` (`SceneComponent.K2_GetComponentToWorld` _array_element) (`self.ExplosionPos`))) (.y (`KismetMathLibrary.InverseTransformLocation` (`SceneComponent.K2_GetComponentToWorld` _array_element) (`self.ExplosionPos`))) (`KismetMathLibrary.FMax` (.z (`KismetMathLibrary.InverseTransformLocation` (`SceneComponent.K2_GetComponentToWorld` _array_element) (`self.ExplosionPos`))) 50.0) (`self.ExplosionRadius`))))
  (`KismetSystemLibrary.Delay` 4.3898)
  (goto _label))

(fn `UserConstructionScript`
  (set `self.StaticMeshArray` (`self.K2_GetComponentsByClass` "/Script/Engine.StaticMeshComponent"))
  (for _array_element (`self.StaticMeshArray`)
    (`PrimitiveComponent.SetCustomPrimitiveDataVector4` _array_element 0 (`KismetMathLibrary.MakeVector4` (.x (`KismetMathLibrary.InverseTransformLocation` (`SceneComponent.GetRelativeTransform` _array_element) (`self.ExplosionPos`))) (.y (`KismetMathLibrary.InverseTransformLocation` (`SceneComponent.GetRelativeTransform` _array_element) (`self.ExplosionPos`))) (.z (`KismetMathLibrary.InverseTransformLocation` (`SceneComponent.GetRelativeTransform` _array_element) (`self.ExplosionPos`))) 100.0))))